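; Edible AI pawn that wanders the level, approaches the player when seen, and can be eaten to raise the player's Hunger value.
; A looping timer picks random reachable destinations, while PawnSensing sightings send it toward the player.
; Overlap shows or fades the EatInteract widget.
; EatCharacterFood adds Hunger in small delayed steps over LoopTimes, caps it at the end, then destroys the actor.
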(event OnSeePawn(PawnSensing)
  (params (Pawn :type Pawn%20Object%20Reference))
  (bind _asthird_person_character (Utilities|Casting|CastToThirdPersonCharacter Pawn))
  (Variables|Default|SetCanSeePlayer true)
  (AI|AIMoveTo self "0, 0, 0" _asthird_person_character 5.0 false
    (:OnSuccess
      _)
    (:OnFail
      _))
  (Variables|Default|SetCanSeePlayer false))

(event Custom|SeePlayer
  (if (Variables|Default|GetCanSeePlayer)
    (CallFunction|MovetoPlayer)
    (else
      (AI|AIMoveTo self (.RandomLocation (AI|Navigation|GetRandomReachablePointinRadius (Transformation|GetActorLocation) 1e+03 0 0)) 0 5.0 false))))

(event Custom|MoveToPlayer
  (AI|AIMoveTo self "0, 0, 0" (stale OnSeePawn(PawnSensing) _asthird_person_character) 5.0 false
    (:OnSuccess
      _)
    (:OnFail
      _))
  (Variables|Default|SetCanSeePlayer false))

(event Custom|EatCharacterFood
  (bind _asthird_person_character (Utilities|Casting|CastToThirdPersonCharacter (Game|GetPlayerCharacter 0)))
  (Variables|/Game/Character/Blueprints/Character/ThirdPersonCharacter.ThirdPersonCharacter_C|SetHunger _asthird_person_character (+ (Variables|/Game/Character/Blueprints/Character/ThirdPersonCharacter.ThirdPersonCharacter_C|GetHunger _asthird_person_character) 0.01) :!label _label)
  (Variables|Default|SetLoopTimes (- (Variables|Default|GetLoopTimes) 1.0))
  (if (<= (Variables|Default|GetLoopTimes) 0.0)
    (if (> (Variables|/Game/Character/Blueprints/Character/ThirdPersonCharacter.ThirdPersonCharacter_C|GetHunger _asthird_person_character) 1.0)
      (Variables|/Game/Character/Blueprints/Character/ThirdPersonCharacter.ThirdPersonCharacter_C|SetHunger _asthird_person_character 1.0))
    (Actor|DestroyActor)
    (else
      (Utilities|FlowControl|Delay 0.034722)
      (goto _label))))

(event EventBeginPlay
  (Utilities|Time|SetTimerbyEvent (delegate Custom|SeePlayer) 3.0 true))

(event Collision|EventActorEndOverlap
  (params (OtherActor :type Actor%20Object%20Reference))
  (Utilities|Casting|CastToThirdPersonCharacter OtherActor)
  (Default|FadeOut (stale Collision|EventActorBeginOverlap _returnvalue)))

(event Collision|EventActorBeginOverlap
  (params (OtherActor :type Actor%20Object%20Reference))
  (Utilities|Casting|CastToThirdPersonCharacter OtherActor)
  (bind _returnvalue (UserInterface|CreateWidget "/Game/UI/EatInteract.EatInteract_C"))
  (UserInterface|Viewport|AddtoViewport _returnvalue 0))

(fn ConstructionScript)