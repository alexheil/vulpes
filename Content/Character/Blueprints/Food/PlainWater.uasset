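; PlainWater is a drinkable water actor that restores the player character's Thirst.
; Character overlap creates a DrinkInteract widget on screen, and leaving fades it out.
; DrinkWater, whose caller is outside this graph, raises Thirst gradually through a Delay-driven loop counted down by LoopTimes.
; When the countdown ends, Thirst above full is clamped, and only in that case does LoopTimes reset.
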(event Custom|DrinkWater
  (bind _asthird_person_character (Utilities|Casting|CastToThirdPersonCharacter (Game|GetPlayerCharacter 0)))
  (Variables|/Game/Character/Blueprints/Character/ThirdPersonCharacter.ThirdPersonCharacter_C|SetThirst _asthird_person_character (+ (Variables|/Game/Character/Blueprints/Character/ThirdPersonCharacter.ThirdPersonCharacter_C|GetThirst _asthird_person_character) 0.01) :!label _label)
  (Variables|Default|SetLoopTimes (- (Variables|Default|GetLoopTimes) 1.0))
  (if (<= (Variables|Default|GetLoopTimes) 0.0)
    (if (> (Variables|/Game/Character/Blueprints/Character/ThirdPersonCharacter.ThirdPersonCharacter_C|GetThirst _asthird_person_character) 1.0)
      (Variables|/Game/Character/Blueprints/Character/ThirdPersonCharacter.ThirdPersonCharacter_C|SetThirst _asthird_person_character 1.0)
      (Variables|Default|SetLoopTimes 1e+02))
    (else
      (Utilities|FlowControl|Delay 0.034722)
      (goto _label))))

(event EventBeginPlay)

(event Collision|EventActorBeginOverlap
  (params (OtherActor :type Actor%20Object%20Reference))
  (Utilities|Casting|CastToThirdPersonCharacter OtherActor)
  (bind _returnvalue (UserInterface|CreateWidget "/Game/UI/DrinkInteract.DrinkInteract_C"))
  (UserInterface|Viewport|AddtoViewport _returnvalue 0))

(event EventTick
  (params (DeltaSeconds :type Float%20%28single-precision%29)))

(event Collision|EventActorEndOverlap
  (params (OtherActor :type Actor%20Object%20Reference))
  (Utilities|Casting|CastToThirdPersonCharacter OtherActor)
  (Default|FadeOut (stale Collision|EventActorBeginOverlap _returnvalue)))

(fn ConstructionScript)