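; Enemy character Blueprint that wanders, chases the player on sight and drains the player's health on contact.
; Pawn sensing sets a sight flag and starts an AI move toward the player, which clears the flag on success or failure.
; A looping timer either repeats the chase or picks a random reachable point nearby.
; Overlap starts a delayed damage loop that has no end-overlap check, so it keeps running after contact ends.
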(event OnSeePawn(PawnSensing)
  (params (Pawn :type Pawn%20Object%20Reference))
  (bind _asthird_person_character (Utilities|Casting|CastToThirdPersonCharacter Pawn))
  (Variables|Default|SetCanSeePlayer true)
  (AI|AIMoveTo self "0, 0, 0" _asthird_person_character 5.0 false
    (:OnSuccess
      _)
    (:OnFail
      _))
  (Variables|Default|SetCanSeePlayer false))

(event Custom|SeePlayer
  (if (Variables|Default|GetCanSeePlayer)
    (CallFunction|MovetoPlayer)
    (else
      (AI|AIMoveTo self (.RandomLocation (AI|Navigation|GetRandomReachablePointinRadius (Transformation|GetActorLocation) 1e+03 0 0)) 0 5.0 false))))

(event Custom|MoveToPlayer
  (AI|AIMoveTo self "0, 0, 0" (stale OnSeePawn(PawnSensing) _asthird_person_character) 5.0 false
    (:OnSuccess
      _)
    (:OnFail
      _))
  (Variables|Default|SetCanSeePlayer false))

(event EventBeginPlay
  (Utilities|Time|SetTimerbyEvent (delegate Custom|SeePlayer) 3.0 true))

(event EventTick
  (params (DeltaSeconds :type Float%20%28single-precision%29)))

(event Collision|EventActorBeginOverlap
  (params (OtherActor :type Actor%20Object%20Reference))
  (bind _asthird_person_character (Utilities|Casting|CastToThirdPersonCharacter OtherActor :!label _label))
  (Variables|/Game/Character/Blueprints/Character/ThirdPersonCharacter.ThirdPersonCharacter_C|SetHealth _asthird_person_character (- (Variables|/Game/Character/Blueprints/Character/ThirdPersonCharacter.ThirdPersonCharacter_C|GetHealth _asthird_person_character) 0.1))
  (Utilities|FlowControl|Delay 0.5)
  (goto _label))

(fn ConstructionScript)